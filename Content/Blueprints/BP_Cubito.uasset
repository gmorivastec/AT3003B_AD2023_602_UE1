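; BP_Cubito is a Blueprint that exercises a simple addition function and on-screen printing, apparently as a practice asset.
; On BeginPlay it prints a Spanish greeting, then calls Sumar twice with fixed inputs and prints each sum, the second with a label.
; Sumar returns the sum of A and B and also prints whether that sum is greater than 5.
; Tick, overlap and the construction script are empty.
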(event `self.ReceiveBeginPlay`
  (`KismetSystemLibrary.PrintString` "Hola amiguitos" true true (struct :`R` 1.0 :`G` 0.496819 :`A` 1.0) 3.0)
  (bind _resultado (`self.Sumar` 3 4))
  (`KismetSystemLibrary.PrintString` (`KismetStringLibrary.Conv_IntToString` _resultado))
  (bind _resultado_2 (`self.Sumar` 2 1))
  (`KismetSystemLibrary.PrintString` (`KismetStringLibrary.Concat_StrStr` "El resultado fue: " (`KismetStringLibrary.Conv_IntToString` _resultado_2)) true true (struct :`G` 0.66 :`B` 1.0 :`A` 1.0) 5.0))

(event `self.ReceiveTick`
  (params (DeltaSeconds :type "Float (single-precision)")))

(fn `Sumar`
  (params (A :type Integer) (B :type Integer))
  (returns (Resultado :type Integer))
  (bind _returnvalue (+ A B))
  (if (> _returnvalue 5)
    (`KismetSystemLibrary.PrintString` "mayor que 5")
    (else
      (`KismetSystemLibrary.PrintString` "menor o igual que 5")))
  (return _returnvalue))

(fn `UserConstructionScript`)